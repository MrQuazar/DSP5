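; BP_Player is the player actor, with Enhanced Input controls for looking around and swimming.
; On BeginPlay it adds the IMC_Swim mapping context to player 0's input subsystem.
; Look actions feed controller yaw and pitch on player pawn 0.
; Propel adds movement input along the camera's forward vector, scaled by PropelStrength and the action value, so movement follows view direction.
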(event `self.ReceiveBeginPlay`
  (`EnhancedInputSubsystemInterface.AddMappingContext` (pcsubsystem `EnhancedInputLocalPlayerSubsystem` (`GameplayStatics.GetPlayerController` 0)) "/Game/Dynamic/Inputs/IMC_Swim.IMC_Swim" 0 (struct)))

(event `EnhancedInput|/Game/Dynamic/Inputs/IA_LookAround`
  (params (ActionValue :type "Vector2D Structure") (ElapsedSeconds :type "Float (double-precision)") (TriggeredSeconds :type "Float (double-precision)") (InputAction :type "InputAction Object Reference" :default "/Game/Dynamic/Inputs/IA_LookAround.IA_LookAround"))
  (:`Triggered`
    (`self.AddControllerYawInput` (`GameplayStatics.GetPlayerPawn` 0) (`KismetMathLibrary.BreakVector2D` ActionValue))))

(event `EnhancedInput|/Game/Dynamic/Inputs/IA_LookUp`
  (params (ActionValue :type "Vector2D Structure") (ElapsedSeconds :type "Float (double-precision)") (TriggeredSeconds :type "Float (double-precision)") (InputAction :type "InputAction Object Reference" :default "/Game/Dynamic/Inputs/IA_LookUp.IA_LookUp"))
  (:`Triggered`
    (`self.AddControllerPitchInput` (`GameplayStatics.GetPlayerPawn` 0) (`KismetMathLibrary.BreakVector2D` ActionValue))))

(event `EnhancedInput|/Game/Dynamic/Inputs/IA_Propel`
  (params (ActionValue :type "Float (double-precision)") (ElapsedSeconds :type "Float (double-precision)") (TriggeredSeconds :type "Float (double-precision)") (InputAction :type "InputAction Object Reference" :default "/Game/Dynamic/Inputs/IA_Propel.IA_Propel"))
  (:`Triggered`
    (`self.AddMovementInput` (`GameplayStatics.GetPlayerPawn` 0) (* (`self.PropelStrength`) (`KismetMathLibrary.GetForwardVector` (`SceneComponent.K2_GetComponentRotation` (`self.Camera`)))) ActionValue false)))

(fn `UserConstructionScript`)