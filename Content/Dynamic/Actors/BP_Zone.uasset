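; BP_Zone is a zone actor meant to shrink over time, apparently as a shrinking play area.
; BeginPlay caches the Zone component's initial scale and location, then starts a fast looping timer calling ShrinkZoneDynamic, which is currently empty.
; An alternative stepped ShrinkZone lowers uniform scale by ScaleTick and reports whether another step stays above MinScale, but its interval timer is disconnected.
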(event `self.ReceiveBeginPlay`
  (bind _zone (`self.Zone`))
  (set `self.InitialScale` (`SceneComponent.K2_GetComponentScale` _zone))
  (set `self.InitialLocation` (`SceneComponent.K2_GetComponentLocation` _zone))
  (`KismetSystemLibrary.K2_SetTimerDelegate` (delegate `DynamicShrinkZone`) 0.01 true))

(event `DynamicShrinkZone`
  (`self.ShrinkZoneDynamic`))

(event `StaticZoneShrink`
  (bind _isshrinkable (`self.ShrinkZone`))
  (if _isshrinkable
    _))

(fn `ShrinkZone`
  (returns (isShrinkable :type Boolean))
  (bind _returnvalue (- (`self.CurrentScale`) (`self.ScaleTick`)))
  (`SceneComponent.SetWorldScale3D` (`self.Zone`) (`KismetMathLibrary.Conv_DoubleToVector` _returnvalue))
  (set `self.CurrentScale` _returnvalue)
  (return (>= _returnvalue (`self.MinScale`))))

(fn `ShrinkZoneDynamic`)

(fn `UserConstructionScript`)